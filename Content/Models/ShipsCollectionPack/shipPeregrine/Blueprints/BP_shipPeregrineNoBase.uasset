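; Placeable Peregrine ship Blueprint (NoBase version) with selectable color variations and no active runtime logic.
; The construction script switches on ColorVariations to apply one of three material sets to the Ship component's wood, cloth and metal slots.
; Variation 2 reuses some of Variation 1's materials, changing only one wood slot and the cloth.
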(event EventBeginPlay)

(event Collision|EventActorBeginOverlap
  (params (OtherActor :type Actor%20Object%20Reference)))

(event EventTick
  (params (DeltaSeconds :type Float%20%28single-precision%29)))

(fn ConstructionScript
  (switch Utilities|FlowControl|Switch|SwitchonE_shipPeregrineVariations (Variables|Default|GetColorVariations)
    (:NewEnumerator0
      (Rendering|Material|SetMaterial (Variables|Default|Getship) 0 "/Game/ShipsCollectionPack/shipPeregrine/Materials/MI_shipPeregrine_woodB_v1.MI_shipPeregrine_woodB_v1")
      (Rendering|Material|SetMaterial (Variables|Default|Getship) 1 "/Game/ShipsCollectionPack/shipPeregrine/Materials/MI_shipPeregrine_woodA_v1.MI_shipPeregrine_woodA_v1")
      (Rendering|Material|SetMaterial (Variables|Default|Getship) 2 "/Game/ShipsCollectionPack/shipPeregrine/Materials/MI_shipPeregrine_cloth_v1.MI_shipPeregrine_cloth_v1")
      (Rendering|Material|SetMaterial (Variables|Default|Getship) 3 "/Game/ShipsCollectionPack/shipPeregrine/Materials/MI_shipPeregrine_metal_v1.MI_shipPeregrine_metal_v1"))
    (:NewEnumerator1
      (Rendering|Material|SetMaterial (Variables|Default|Getship) 0 "/Game/ShipsCollectionPack/shipPeregrine/Materials/MI_shipPeregrine_woodB_v1.MI_shipPeregrine_woodB_v1")
      (Rendering|Material|SetMaterial (Variables|Default|Getship) 1 "/Game/ShipsCollectionPack/shipPeregrine/Materials/MI_shipPeregrine_woodA_v2.MI_shipPeregrine_woodA_v2")
      (Rendering|Material|SetMaterial (Variables|Default|Getship) 2 "/Game/ShipsCollectionPack/shipPeregrine/Materials/MI_shipPeregrine_cloth_v2.MI_shipPeregrine_cloth_v2")
      (Rendering|Material|SetMaterial (Variables|Default|Getship) 3 "/Game/ShipsCollectionPack/shipPeregrine/Materials/MI_shipPeregrine_metal_v1.MI_shipPeregrine_metal_v1"))
    (:NewEnumerator2
      (Rendering|Material|SetMaterial (Variables|Default|Getship) 0 "/Game/ShipsCollectionPack/shipPeregrine/Materials/MI_shipPeregrine_woodB_v3.MI_shipPeregrine_woodB_v3")
      (Rendering|Material|SetMaterial (Variables|Default|Getship) 1 "/Game/ShipsCollectionPack/shipPeregrine/Materials/MI_shipPeregrine_woodA_v3.MI_shipPeregrine_woodA_v3")
      (Rendering|Material|SetMaterial (Variables|Default|Getship) 2 "/Game/ShipsCollectionPack/shipPeregrine/Materials/MI_shipPeregrine_cloth_v3.MI_shipPeregrine_cloth_v3")
      (Rendering|Material|SetMaterial (Variables|Default|Getship) 3 "/Game/ShipsCollectionPack/shipPeregrine/Materials/MI_shipPeregrine_metal_v3.MI_shipPeregrine_metal_v3"))))