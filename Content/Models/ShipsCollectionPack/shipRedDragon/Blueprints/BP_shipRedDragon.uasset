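; Red Dragon ship actor from the ShipsCollectionPack with selectable color variations.
; The construction script switches on the ColorVariations setting and assigns the matching body and wood material instances to the two material slots of the Ship mesh, for one of three variants.
; It has no runtime logic, as the event graph holds only disabled default events.
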(event EventBeginPlay)

(event Collision|EventActorBeginOverlap
  (params (OtherActor :type Actor%20Object%20Reference)))

(event EventTick
  (params (DeltaSeconds :type Float%20%28single-precision%29)))

(fn ConstructionScript
  (switch Utilities|FlowControl|Switch|SwitchonE_shipRedDragonVariations (Variables|Default|GetColorVariations)
    (:NewEnumerator0
      (Rendering|Material|SetMaterial (Variables|Default|Getship) 1 "/Game/ShipsCollectionPack/shipRedDragon/Materials/MI_shipRedDragon_v1.MI_shipRedDragon_v1")
      (Rendering|Material|SetMaterial (Variables|Default|Getship) 0 "/Game/ShipsCollectionPack/shipRedDragon/Materials/MI_shipRedDragon_wood_v1.MI_shipRedDragon_wood_v1"))
    (:NewEnumerator1
      (Rendering|Material|SetMaterial (Variables|Default|Getship) 1 "/Game/ShipsCollectionPack/shipRedDragon/Materials/MI_shipRedDragon_v2.MI_shipRedDragon_v2")
      (Rendering|Material|SetMaterial (Variables|Default|Getship) 0 "/Game/ShipsCollectionPack/shipRedDragon/Materials/MI_shipRedDragon_wood_v2.MI_shipRedDragon_wood_v2"))
    (:NewEnumerator2
      (Rendering|Material|SetMaterial (Variables|Default|Getship) 1 "/Game/ShipsCollectionPack/shipRedDragon/Materials/MI_shipRedDragon_v3.MI_shipRedDragon_v3")
      (Rendering|Material|SetMaterial (Variables|Default|Getship) 0 "/Game/ShipsCollectionPack/shipRedDragon/Materials/MI_shipRedDragon_wood_v3.MI_shipRedDragon_wood_v3"))))