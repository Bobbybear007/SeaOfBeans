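; BP_shipMasterhandNoBase is a Masterhand ship prop from the ShipsCollectionPack with selectable color variations.
; The construction script switches on ColorVariations and assigns the matching wood and cloth material instances to the Ship component's first two material slots.
; The event graph holds only disabled default events, so the asset has no runtime logic of its own.
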(event EventBeginPlay)

(event Collision|EventActorBeginOverlap
  (params (OtherActor :type Actor%20Object%20Reference)))

(event EventTick
  (params (DeltaSeconds :type Float%20%28single-precision%29)))

(fn ConstructionScript
  (switch Utilities|FlowControl|Switch|SwitchonE_shipMasterhandVariations (Variables|Default|GetColorVariations)
    (:NewEnumerator0
      (Rendering|Material|SetMaterial (Variables|Default|GetShip) 0 "/Game/ShipsCollectionPack/shipMasterhand/Materials/MI_shipMasterhand_wood_v1.MI_shipMasterhand_wood_v1")
      (Rendering|Material|SetMaterial (Variables|Default|GetShip) 1 "/Game/ShipsCollectionPack/shipMasterhand/Materials/MI_shipMasterhand_cloth_v1.MI_shipMasterhand_cloth_v1"))
    (:NewEnumerator1
      (Rendering|Material|SetMaterial (Variables|Default|GetShip) 0 "/Game/ShipsCollectionPack/shipMasterhand/Materials/MI_shipMasterhand_wood_v2.MI_shipMasterhand_wood_v2")
      (Rendering|Material|SetMaterial (Variables|Default|GetShip) 1 "/Game/ShipsCollectionPack/shipMasterhand/Materials/MI_shipMasterhand_cloth_v2.MI_shipMasterhand_cloth_v2"))
    (:NewEnumerator2
      (Rendering|Material|SetMaterial (Variables|Default|GetShip) 0 "/Game/ShipsCollectionPack/shipMasterhand/Materials/MI_shipMasterhand_wood_v3.MI_shipMasterhand_wood_v3")
      (Rendering|Material|SetMaterial (Variables|Default|GetShip) 1 "/Game/ShipsCollectionPack/shipMasterhand/Materials/MI_shipMasterhand_cloth_v3.MI_shipMasterhand_cloth_v3"))))